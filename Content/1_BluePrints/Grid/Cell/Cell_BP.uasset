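; Grid cell actor for unit movement, attack and spawn targeting, registering itself with the level's Grid.
; On BeginPlay it box-traces for four axis-aligned neighbours and spawns an attached GridCell, whose state reflects any character on top.
; Targeting swaps the cube material by selection type and updates the GridCell, which also grows on cursor hover.
; A downward trace finds the occupant, which feeds the walkability check alongside a layer comparison.
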(event OnBeginCursorOver(Cube)
  (params (TouchedComponent :type Primitive%20Component%20Object%20Reference))
  (bind _attached_gridcell (Variables|Default|GetAttached%20GridCell))
  (Default|SetSize _attached_gridcell (+ (Variables|/Game/1_BluePrints/Graphics/Grid/GridCell.GridCell_C|GetActualSize _attached_gridcell) 0.1)))

(event OnEndCursorOver(Cube)
  (params (TouchedComponent :type Primitive%20Component%20Object%20Reference))
  (bind _attached_gridcell (Variables|Default|GetAttached%20GridCell))
  (Default|SetSize _attached_gridcell (Variables|/Game/1_BluePrints/Graphics/Grid/GridCell.GridCell_C|GetActualSize _attached_gridcell)))

(event EventBeginPlay
  (bind _returnvalue (Transformation|GetActorLocation))
  (bind (_x _y) (Math|Vector|BreakVector _returnvalue))
  (bind _returnvalue_2 (Actor|GetActorOfClass "/Game/1_BluePrints/Grid/Grid.Grid_C"))
  (bind _output_get (Variables|Default|SetGrid _returnvalue_2))
  (Default|RegisterCell _output_get self)
  (CallFunction|UpdateNeigbours)
  (Variables|Default|SetBase%20Material (Utilities|Array|Get(acopy) (Rendering|Material|GetMaterials (Variables|Default|GetCube))))
  (bind _returnvalue_3 (Game|SpawnActorfromClass "/Game/1_BluePrints/Graphics/Grid/GridCell.GridCell_C" (Transformation|GetActorTransform) "Undefined" 0 0))
  (Transformation|SetActorLocation _returnvalue_3 (Math|Vector|MakeVector (+ _x (/ (.X (Math|Vector|BreakVector (Variables|/Game/1_BluePrints/Grid/Grid.Grid_C|GetCellSize (Variables|Default|GetGrid)))) 2.0)) (+ _y (/ (.X (Math|Vector|BreakVector (Variables|/Game/1_BluePrints/Grid/Grid.Grid_C|GetCellSize (Variables|Default|GetGrid)))) 2.0)) 0.0) false false)
  (bind _output_get_2 (Variables|Default|SetAttached%20GridCell _returnvalue_3))
  (Default|SetParentCell _output_get_2 self)
  (bind _top_object (CallFunction|GetTopObject))
  (Utilities|Casting|CastToTopDownCharacter_Abstact _top_object
    (:then
      (Variables|/Game/1_BluePrints/Graphics/Grid/GridCell.GridCell_C|SetCurrentState (Variables|Default|GetAttached%20GridCell) "NewEnumerator1")
      (Default|SetSize (Variables|Default|GetAttached%20GridCell) "0.800000,0.800000,0.800000")
      (Variables|/Game/1_BluePrints/Graphics/Grid/GridCell.GridCell_C|SetNewSize (Variables|Default|GetAttached%20GridCell) "0.800000,0.800000,0.800000")
      (Variables|/Game/1_BluePrints/Graphics/Grid/GridCell.GridCell_C|SetActualSize (Variables|Default|GetAttached%20GridCell) "0.800000,0.800000,0.800000"))
    (:CastFailed
      (Variables|/Game/1_BluePrints/Graphics/Grid/GridCell.GridCell_C|SetCurrentState (Variables|Default|GetAttached%20GridCell) "NewEnumerator0")))
  (Default|CallOnCellUpdate))

(event Collision|EventActorBeginOverlap
  (params (OtherActor :type Actor%20Object%20Reference)))

(event EventTick
  (params (DeltaSeconds :type Float%20%28single-precision%29))
  (if (Variables|Default|GetDebug)
    (Development|PrintString (Utilities|String|ToString(Integer) (Utilities|Array|Length (Variables|Default|GetNeigbours))) true true "(R=0.000000,G=0.660000,B=1.000000,A=1.000000)" 0.0)))

(fn ConstructionScript)

(fn GetNeigbours
  (return (Variables|Default|GetNeigbours)))

(fn UpdateNeigbours
  (bind _returnvalue (Transformation|GetActorRotation))
  (bind _returnvalue_2 (Transformation|GetActorLocation))
  (bind _grid (Variables|Default|GetGrid))
  (bind _neigbours (Variables|Default|GetNeigbours))
  (bind _grid_2 (Variables|Default|GetGrid))
  (bind _neigbours_2 (Variables|Default|GetNeigbours))
  (bind _cube (Variables|Default|GetCube))
  (bind _cellsize (Variables|/Game/1_BluePrints/Grid/Grid.Grid_C|GetCellSize _grid))
  (bind _ia_step_height (Variables|/Game/1_BluePrints/Grid/Grid.Grid_C|GetIA%20Step%20height _grid))
  (bind _cellsize_2 (Variables|/Game/1_BluePrints/Grid/Grid.Grid_C|GetCellSize _grid_2))
  (bind _relativelocation (Variables|/Script/Engine.SceneComponent|GetRelativeLocation _cube))
  (bind _returnvalue_3 (+ (.z _cellsize) _ia_step_height))
  (bind _returnvalue_4 (/ (Math|Vector|MakeVector (.x _cellsize) (.y _cellsize) _returnvalue_3) 2.1))
  (Utilities|Array|Clear (Variables|Default|GetNeigbours))
  (bind _outactors (Actor|GetAllActorsOfClass "/Script/Engine.Character"))
  (for _index (range 0 3)
    (Utilities|FlowControl|Sequence
      (:then_0
        (switch int _index
          (:Default
            (LocalVariables|SetBoxTraceCenter (+ _returnvalue_2 (Math|Vector|MakeVector (.x _cellsize_2) 0.0 0.0) _relativelocation) :!label _label))
          (:0
            (goto _label))
          (:1
            (LocalVariables|SetBoxTraceCenter (+ _returnvalue_2 (Math|Vector|MakeVector 0.0 (.y _cellsize_2) 0.0) _relativelocation)))
          (:2
            (LocalVariables|SetBoxTraceCenter (+ _returnvalue_2 (Math|Vector|MakeVector (* -1 (.x _cellsize_2)) 0.0 0.0) _relativelocation)))
          (:3
            (LocalVariables|SetBoxTraceCenter (+ _returnvalue_2 (Math|Vector|MakeVector 0.0 (* -1 (.y _cellsize_2)) 0.0) _relativelocation)))))
      (:then_1
        (if (Variables|Default|GetDebug)
          (bind (_outhit _returnvalue_5) (Collision|BoxTraceByChannel (LocalVariables|GetBoxTraceCenter) (LocalVariables|GetBoxTraceCenter) _returnvalue_4 _returnvalue "TraceTypeQuery1" false _outactors "Persistent"))
          (if _returnvalue_5
            (bind _ascell_bp (Utilities|Casting|CastToCell_BP (.HitActor (Collision|BreakHitResult _outhit))))
            (Utilities|Array|AddUnique _neigbours _ascell_bp)
            (else
              (Utilities|Array|Add _neigbours 0)))
          (else
            (bind (_outhit_2 _returnvalue_6) (Collision|BoxTraceByChannel (LocalVariables|GetBoxTraceCenter) (LocalVariables|GetBoxTraceCenter) _returnvalue_4 _returnvalue "TraceTypeQuery1" false _outactors "None"))
            (if _returnvalue_6
              (bind _ascell_bp_2 (Utilities|Casting|CastToCell_BP (.HitActor (Collision|BreakHitResult _outhit_2))))
              (Utilities|Array|AddUnique _neigbours_2 _ascell_bp_2)
              (else
                (Utilities|Array|Add _neigbours_2 0)))))))))

(fn GetRightNeigbour
  (return (Utilities|Array|Get(acopy) (Variables|Default|GetNeigbours) 1)))

(fn GetTopNeigbour
  (return (Utilities|Array|Get(acopy) (Variables|Default|GetNeigbours))))

(fn GetLeftNeigbour
  (return (Utilities|Array|Get(acopy) (Variables|Default|GetNeigbours) 3)))

(fn GetBottomNeigbour
  (return (Utilities|Array|Get(acopy) (Variables|Default|GetNeigbours) 2)))

(fn CompareLayer
  (params (Unit%20Layer :type Integer))
  (return (== Unit%20Layer (Variables|Default|GetLayer))))

(fn SetTargetable
  (params (SelectionType :type SelectionType%20Enum :default "NewEnumerator0"))
  (Variables|/Game/1_BluePrints/Graphics/Grid/GridCell.GridCell_C|SetCurrentState (Variables|Default|GetAttached%20GridCell) "NewEnumerator2")
  (Variables|Default|SetSelectionType SelectionType)
  (switch Utilities|FlowControl|Switch|SwitchonSelectionType SelectionType
    (:NewEnumerator0
      (Rendering|Material|SetMaterial (Variables|Default|GetCube) 0 (Variables|Default|GetHiglight%20Move%20Material)))
    (:NewEnumerator1
      (Rendering|Material|SetMaterial (Variables|Default|GetCube) 0 (Variables|Default|GetHighlight%20Attack%20Material%20)))
    (:NewEnumerator2
      (Rendering|Material|SetMaterial (Variables|Default|GetCube) 0 (Variables|Default|GetHiglight%20Spawn%20Material))))
  (Variables|Default|SetIsTargetable true)
  (Utilities|Array|AddUnique (Variables|/Game/1_BluePrints/Grid/Grid.Grid_C|GetHighlightedCells (Variables|Default|GetGrid)) self)
  (Default|CallOnCellUpdate))

(fn SetUntargetable
  (Rendering|Material|SetMaterial (Variables|Default|GetCube) 0 (Variables|Default|GetBase%20Material))
  (Variables|Default|SetIsTargetable false)
  (Default|ResetCell (Variables|Default|GetAttached%20GridCell)))

(fn GetTopObject
  (bind _returnvalue (Transformation|GetActorLocation))
  (bind _grid (Variables|Default|GetGrid))
  (bind _cellsize (Variables|/Game/1_BluePrints/Grid/Grid.Grid_C|GetCellSize _grid))
  (bind _returnvalue_2 (/ _cellsize 2.0))
  (bind _returnvalue_3 (+ _returnvalue _returnvalue_2))
  (bind _outhit (Collision|BoxTraceByChannel (+ _returnvalue_3 "0, 0,1000.000000") _returnvalue_3 "1.000000,1.000000,50.000000" "0, 0, 0" "TraceTypeQuery1" false 0 "None"))
  (return (.HitActor (Collision|BreakHitResult _outhit))))

(fn IsWalkable
  (params (Layer :type Integer))
  (bind _top_object (CallFunction|GetTopObject))
  (return (and (== _top_object 0) (== Layer (Variables|Default|GetLayer)))))